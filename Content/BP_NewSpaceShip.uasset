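; Player spaceship with touch-joystick steering, constant forward drift and damage feedback.
; Tick offsets the Body along negative local X to suit the backward-facing model, using teleport.
; Axis inputs apply pitch and yaw torque; with both released, angular velocity lerps toward zero for smooth deceleration.
; Any damage lowers Health and plays a random camera shake and hit sound, plus an explosion effect if caused by a damaging body.
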(event `TakeDamageEvent` :!signature `self.OnTakeAnyDamage`
  (params (DamagedActor :type "Actor Object Reference") (Damage :type "Float (double-precision)") (DamageType :type "DamageType Object Reference") (InstigatedBy :type "Controller Object Reference") (DamageCauser :type "Actor Object Reference"))
  (bind _var_controller (`self.var_controller`))
  ;[1 1 1] Taking damage function
  (set `self.Health` (- (`self.Health`) Damage))
  ;[1 1 1] Deciding the camera shake to play
  (switch `int` (`KismetMathLibrary.RandomIntegerInRange` 0 1)
    (:`0`
      (`PlayerController.ClientStartCameraShake` :`self` _var_controller :`Shake` "/Game/CameraShakes_Kshitij/BP_HitShake1_Kshitij.BP_HitShake1_Kshitij_C"))
    (:`1`
      (`PlayerController.ClientStartCameraShake` :`self` _var_controller :`Shake` "/Game/CameraShakes_Kshitij/BP_HitShake2_Kshitij.BP_HitShake2_Kshitij_C")))
  (`AudioComponent.Play` (`self.HitObjectSound`) 0.0)
  (if (== (`GameplayStatics.GetObjectClass` DamageCauser) "/Game/DamagingBodies_Kshitij/BP_DamagingBodies_Kshitij.BP_DamagingBodies_Kshitij_C")
    (`ActorComponent.Activate` (`self.HitEffectExplosion`) false)
    (else
      (`KismetSystemLibrary.PrintString` "Not damaging body"))))

(event `self.ReceiveBeginPlay`
  (bind _returnvalue (`GameplayStatics.GetPlayerController` 0))
  ;[1 1 1] Creating the touch interface and storing in a variable, binding the take damage function
  (`PlayerController.ActivateTouchInterface` _returnvalue "/Game/CustomJoystick_Kshitij.CustomJoystick_Kshitij")
  (set `self.var_controller` _returnvalue)
  (add `self.OnTakeAnyDamage` (delegate `TakeDamageEvent`)))

(event `self.ReceiveTick`
  (params (DeltaSeconds :type "Float (single-precision)"))
  ;[1 1 1] Adding a default forward movement to the ship
  (`SceneComponent.K2_AddLocalOffset` (`self.Body`) (`KismetMathLibrary.MakeVector` (* DeltaSeconds (* (`self.ForwardMovementFactor`) -1.0))) false true))

(event `InputAxis|ForwardBack`
  (params (AxisValue :type "Float (single-precision)"))
  (bind _body (`self.Body`))
  ;[1 1 1] Handling the up and down movement,enabling simulate physics if input is applied
  (if (== AxisValue 0.0)
    (set `self.bForward` false)
    (if (not (`self.bLeft`))
      ;[1 1 1] Slowly lerping the velocity, towards zero, to give it a smooth transition,will be used in case of deceleration
      (`PrimitiveComponent.SetPhysicsAngularVelocityInDegrees` _body (`KismetMathLibrary.VLerp` (`PrimitiveComponent.GetPhysicsAngularVelocityInDegrees` _body "None") (0.0 0.0 0.0) (* (`GameplayStatics.GetWorldDeltaSeconds`) (`self.DecelerationFac`))) false "None" :!label _label))
    (else
      (set `self.bForward` true)
      (`PrimitiveComponent.AddTorqueInDegrees` (`self.Body`) (* (`self.GetActorRightVector`) (* 40 AxisValue)) "None" true))))

(event `InputAxis|RightLeft`
  (params (AxisValue :type "Float (single-precision)"))
  ;[1 1 1] Handling the left and right movement,enabling simulate physics if input is applied
  (if (== AxisValue 0.0)
    (set `self.bLeft` false)
    (if (not (`self.bForward`))
      (goto _label))
    (else
      (set `self.bLeft` true)
      (`PrimitiveComponent.AddTorqueInDegrees` (`self.Body`) (* (`self.GetActorUpVector`) (* 40 AxisValue)) "None" true))))

(fn `UserConstructionScript`)