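; Paladin enemy that fights the ThirdPersonCharacter when something overlaps its Box.
; If the overlapping player is slashing, it sets Attacked, plays a hit-backwards death animation and is destroyed after a delay.
; The same overlap starts a melee montage and, unless Attacked, removes one player Health.
; At zero Health it calls the player's Death and pauses the game after a delay.
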(event `self.Box.OnComponentBeginOverlap`
  (params (OverlappedComponent :type "PrimitiveComponent Object Reference") (OtherActor :type "Actor Object Reference") (OtherComp :type "PrimitiveComponent Object Reference") (OtherBodyIndex :type Integer) (bFromSweep :type Boolean) (SweepResult :type "HitResult Structure (by ref)"))
  (`|ExecutionSequence`
    (:`then_0`
      ;[1 1 1] Death
      (bind _asthird_person_character (cast `/Game/ThirdPersonBP/Blueprints/ThirdPersonCharacter` OtherActor))
      (if (`/Game/ThirdPersonBP/Blueprints/ThirdPersonCharacter.SlashSword` _asthird_person_character)
        (set `self.Attacked` true)
        (`self.death`)
        (`KismetSystemLibrary.Delay` 1.0)
        (`self.K2_DestroyActor`)
        (set `self.Attacked` false)))
    (:`then_1`
      ;[1 1 1] Attack
      (`|PlayMontage` (`self.paladin_prop_j_nordstrom`) "/Game/Assets/NewAssets/Standing_Melee_Attack_Horizontal_Anim_Montage.Standing_Melee_Attack_Horizontal_Anim_Montage"
        (:`then`
          (if (not (`self.Attacked`))
            (bind _asthird_person_character_2 (cast `/Game/ThirdPersonBP/Blueprints/ThirdPersonCharacter` OtherActor))
            (set `/Game/ThirdPersonBP/Blueprints/ThirdPersonCharacter.health` (- (`/Game/ThirdPersonBP/Blueprints/ThirdPersonCharacter.health` _asthird_person_character_2) 1) _asthird_person_character_2)
            (if (== (`/Game/ThirdPersonBP/Blueprints/ThirdPersonCharacter.health` _asthird_person_character_2) 0)
              (`/Game/ThirdPersonBP/Blueprints/ThirdPersonCharacter.Death` _asthird_person_character_2)
              (`KismetSystemLibrary.Delay` 2.0)
              (`GameplayStatics.SetGamePaused` true))))))))

(fn `death`
  (`SkeletalMeshComponent.PlayAnimation` (`self.paladin_prop_j_nordstrom`) "/Game/Assets/NewAssets/Getting_Hit_Backwards.Getting_Hit_Backwards" false))

(fn `UserConstructionScript`)