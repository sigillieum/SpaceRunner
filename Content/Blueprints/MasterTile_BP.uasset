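; Track tile for a three-lane runner that fills itself with random obstacles and pickups on BeginPlay via child actor components.
; Construction caches lane transforms for obstacles; the pickup transform array has its own setter, which is never called here.
; Each branch in the chance chains rolls a fresh random number.
; Player overlap with the box asks the game mode for another tile, then destroys this one after a short delay.
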(event `self.ReceiveBeginPlay`
  (`self.Spawn Obstcales`)
  (`self.Spawn Pickups`))

(event `self.Box.OnComponentBeginOverlap`
  (params (OverlappedComponent :type "PrimitiveComponent Object Reference") (OtherActor :type "Actor Object Reference") (OtherComp :type "PrimitiveComponent Object Reference") (OtherBodyIndex :type Integer) (bFromSweep :type Boolean) (SweepResult :type "HitResult Structure (by ref)"))
  (cast `/Game/ThirdPersonBP/Blueprints/ThirdPersonCharacter` OtherActor)
  (bind _asthird_person_game_mode (cast `/Game/ThirdPersonBP/Blueprints/ThirdPersonGameMode` (`GameplayStatics.GetGameMode`)))
  (`/Game/ThirdPersonBP/Blueprints/ThirdPersonGameMode.SpawnTile` _asthird_person_game_mode)
  (set `self.destory` true)
  (`KismetSystemLibrary.Delay` 0.5)
  (`self.K2_DestroyActor`))

(fn `GetArrow`
  (returns (NewParam :type "Transform Structure"))
  (return (`SceneComponent.K2_GetComponentToWorld` (`self.SpawnPoint`))))

(fn `Set spawn obstcales location`
  (set `self.SpawnObstaclesLocation` (`|MakeArray` (`SceneComponent.GetRelativeTransform` (`self.Lane0`)) (`SceneComponent.GetRelativeTransform` (`self.Lane1`)) (`SceneComponent.GetRelativeTransform` (`self.Lane2`)))))

(fn `Spawn Obstcales`
  (bind _returnvalue (`KismetMathLibrary.RandomFloatInRange` 0.0 1.0))
  (if (`KismetMathLibrary.InRange_FloatFloat` _returnvalue 0.0 0.25)
    (`AddComponent|NODE_AddChildActorComponent-1` :`RelativeTransform` (`|GetArrayItem` (`self.SpawnObstaclesLocation`) (`KismetMathLibrary.RandomIntegerInRange` 0 2)))
    (elif (`KismetMathLibrary.InRange_FloatFloat` _returnvalue 0.25 0.5)
      (`AddComponent|NODE_AddChildActorComponent-2` :`RelativeTransform` (`|GetArrayItem` (`self.SpawnObstaclesLocation`) (`KismetMathLibrary.RandomIntegerInRange` 0 2)))
      (elif (`KismetMathLibrary.InRange_FloatFloat` _returnvalue 0.5 0.75)
        (`AddComponent|NODE_AddChildActorComponent-3` :`RelativeTransform` (`|GetArrayItem` (`self.SpawnObstaclesLocation`) (`KismetMathLibrary.RandomIntegerInRange` 0 1)))))))

(fn `Spawn Pickups`
  (bind _returnvalue (`KismetMathLibrary.RandomFloatInRange` 0.0 1.0))
  (if (`KismetMathLibrary.InRange_FloatFloat` _returnvalue 0.0 0.4)
    ;[1 1 1] Coin Pickups
    (for _ (range (+ (`KismetMathLibrary.RandomIntegerInRange` 0 5) 1))
      (`AddComponent|NODE_AddChildActorComponent-5` :`RelativeTransform` (`|GetArrayItem` (`self.SpawnPickupsLocation`) (`KismetMathLibrary.RandomIntegerInRange` 0 2))))
    (elif (`KismetMathLibrary.InRange_FloatFloat` _returnvalue 0.4 0.8)
      ;[1 1 1] Gear Pickups
      (for _ (range (+ (`KismetMathLibrary.RandomIntegerInRange` 0 5) 1))
        (`AddComponent|NODE_AddChildActorComponent-6` :`RelativeTransform` (`|GetArrayItem` (`self.SpawnPickupsLocation`) (`KismetMathLibrary.RandomIntegerInRange` 0 2))))
      (elif (`KismetMathLibrary.InRange_FloatFloat` _returnvalue 0.8 0.9)
        ;[1 1 1] Magnet Pickups
        (for _ (range (+ (`KismetMathLibrary.RandomIntegerInRange` 0 5) 1))
          (`AddComponent|NODE_AddChildActorComponent-7` :`RelativeTransform` (`|GetArrayItem` (`self.SpawnPickupsLocation`) (`KismetMathLibrary.RandomIntegerInRange` 0 2))))
        (elif (`KismetMathLibrary.InRange_FloatFloat` _returnvalue 0.9)
          ;[1 1 1] Magnet Pickups
          (for _ (range (+ (`KismetMathLibrary.RandomIntegerInRange` 0 5) 1))
            (`AddComponent|NODE_AddChildActorComponent-8` :`RelativeTransform` (`|GetArrayItem` (`self.SpawnPickupsLocation`) (`KismetMathLibrary.RandomIntegerInRange` 0 2)))))))))

(fn `Spawn Pickups Loocation`
  (set `self.SpawnPickupsLocation` (`|MakeArray` (`SceneComponent.K2_GetComponentToWorld` (`self.pickup0`)) (`SceneComponent.K2_GetComponentToWorld` (`self.pickup1`)) (`SceneComponent.K2_GetComponentToWorld` (`self.pickup2`)))))

(fn `UserConstructionScript`
  (`self.Set spawn obstcales location`))