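; Runner coin pickup actor that credits RunnerCharacter through AddCoin.
; Overlapping the Dogecoin component awards the coin and destroys the actor unless it is already marked Used.
; With the magnet active, overlapping the Sphere awards immediately, marks it Used, and destroys it after a short delay.
; Meanwhile a timeline sets its location to world origin; the VInterpTo toward the player is unconnected.
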(event `self.dogecoin.OnComponentBeginOverlap`
  (params (OverlappedComponent :type "PrimitiveComponent Object Reference") (OtherActor :type "Actor Object Reference") (OtherComp :type "PrimitiveComponent Object Reference") (OtherBodyIndex :type Integer) (bFromSweep :type Boolean) (SweepResult :type "HitResult Structure (by ref)"))
  (bind _asrunner_character (cast `/Game/Blueprints/RunnerFolder/RunnerCharacter` OtherActor))
  (if (not (`self.used`))
    (`/Game/Blueprints/RunnerFolder/RunnerCharacter.AddCoin` _asrunner_character)
    (`self.K2_DestroyActor`)))

(event `self.Sphere.OnComponentBeginOverlap`
  (params (OverlappedComponent :type "PrimitiveComponent Object Reference") (OtherActor :type "Actor Object Reference") (OtherComp :type "PrimitiveComponent Object Reference") (OtherBodyIndex :type Integer) (bFromSweep :type Boolean) (SweepResult :type "HitResult Structure (by ref)"))
  (bind _asrunner_character (cast `/Game/Blueprints/RunnerFolder/RunnerCharacter` OtherActor))
  (if (`/Game/Blueprints/RunnerFolder/RunnerCharacter.MagnetActive` _asrunner_character)
    (`|ExecutionSequence`
      (:`then_0`
        (`/Game/Blueprints/RunnerFolder/RunnerCharacter.AddCoin` _asrunner_character)
        (set `self.used` true)
        (`KismetSystemLibrary.Delay` 0.5)
        (`self.K2_DestroyActor`)
        (set `self.used` false))
      (:`then_1`
        (`Timeline|Timeline_0` :!via `PlayFromStart`
          (:`Update`
            (`self.K2_SetActorLocation` (0.0 0.0 0.0))))))))

(fn `UserConstructionScript`)